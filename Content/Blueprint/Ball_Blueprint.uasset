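; Ball actor that bounces around inside an invisible axis-aligned box centered on the world origin.
; Each Tick it tests its location against fixed bounds and flips its ProjectileMovementComponent velocity on any axis at or beyond them.
; The flip is branchless per axis, converting the out-of-bounds boolean into a sign multiplier without checking travel direction.
; BeginPlay creates a dynamic instance of BallMaterial, which the graph does not modify further.
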(event EventTick
  (params (DeltaSeconds :type Float%20%28single-precision%29))
  (bind _returnvalue (Transformation|GetActorLocation))
  (bind _returnvalue_2 (Actor|GetComponentbyClass "/Script/Engine.ProjectileMovementComponent"))
  (bind (_x _y _z) (Math|Vector|BreakVector _returnvalue))
  (bind _returnvalue_3 (>= _z 5e+02))
  (bind _returnvalue_4 (>= _x 5e+02))
  (bind _returnvalue_5 (>= _y 5e+02))
  (bind _returnvalue_6 (<= _z -5e+02))
  (bind _returnvalue_7 (<= _x -5e+02))
  (bind _returnvalue_8 (<= _y -5e+02))
  (bind _returnvalue_9 (or _returnvalue_4 _returnvalue_7))
  (bind _returnvalue_10 (or _returnvalue_3 _returnvalue_6))
  (bind _returnvalue_11 (or _returnvalue_5 _returnvalue_8))
  (if (Math|Boolean|ORBoolean _returnvalue_9 _returnvalue_11 _returnvalue_10)
    (Variables|/Script/Engine.MovementComponent|SetVelocity _returnvalue_2 (* (Variables|/Script/Engine.MovementComponent|GetVelocity _returnvalue_2) (Math|Vector|MakeVector (Math|Conversions|ToFloat(Integer) (+ (* (Math|Conversions|ToInteger(Boolean) _returnvalue_9) -2) 1)) (Math|Conversions|ToFloat(Integer) (+ (* (Math|Conversions|ToInteger(Boolean) _returnvalue_11) -2) 1)) (Math|Conversions|ToFloat(Integer) (+ (* (Math|Conversions|ToInteger(Boolean) _returnvalue_10) -2) 1)))))))

(event EventBeginPlay
  (Rendering|Material|CreateDynamicMaterialInstance "/Game/Blueprint/BallMaterial.BallMaterial" :!class /Script/Engine.KismetMaterialLibrary))

(event Collision|EventActorBeginOverlap
  (params (OtherActor :type Actor%20Object%20Reference)))

(fn ConstructionScript)