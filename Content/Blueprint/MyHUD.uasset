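; HUD Blueprint that displays the player and AI scores, both starting at 3, and handles the game-over state.
; DrawHUD draws the scores on the left and right of the viewport and compares both against 1.
; It shows red GAME OVER text and pauses when the player drops below 1, or the AI does while the player is above 1.
; Nothing in this graph changes the scores after BeginPlay.
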(event EventBeginPlay
  (Variables|Default|SetPlayerScore 3)
  (Variables|Default|SetAiScore 3))

(event EventDrawHUD
  (params (SizeX :type Integer) (SizeY :type Integer))
  (bind _playerscore (Variables|Default|GetPlayerScore))
  (bind _aiscore (Variables|Default|GetAiScore))
  (HUD|DrawText (Utilities|String|ToString(Integer) _playerscore) "(R=0,G=0,B=0,A=1)" 5e+01 0.0 "/Game/ConcertOneLarge.ConcertOneLarge" 1.0 false)
  (HUD|DrawText (Utilities|String|ToString(Integer) _aiscore) "(R=0,G=0,B=0,A=1)" (- (.X (Math|Vector2D|BreakVector2D (Viewport|GetViewportSize))) 175.0) 0.0 "/Game/ConcertOneLarge.ConcertOneLarge" 1.0 false)
  (Math|Integer|CompareInt _playerscore 1
    (:>
      (Math|Integer|CompareInt _aiscore 1
        (:<
          (HUD|DrawText "GAME OVER" "(R=0.862745,G=0.007843,B=0.000000,A=1.000000)" 5e+01 5e+01 "/Game/ConcertOneLarge.ConcertOneLarge" 1.0 false)
          (Game|SetGamePaused true))))
    (:<
      (HUD|DrawText "GAME OVER" "(R=0.862745,G=0.007843,B=0.000000,A=1.000000)" 5e+01 5e+01 "/Game/ConcertOneLarge.ConcertOneLarge" 0.8 false)
      (Game|SetGamePaused true))))

(fn ConstructionScript)